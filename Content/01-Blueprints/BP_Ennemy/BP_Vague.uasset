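; BP_Vague is an enemy wave spawner that sends BP_Ennemy pawns out from its Billboard location.
; The T key starts spawning through a self-calling, delayed LoopWithDelay event.
; WaveEnd checks the remaining count, enlarges the next wave and relaunches it after a pause.
; ResetByPortail, also bound to R, restores the starting wave size, destroys all enemies and sets a flag that blocks the next wave.
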(event Custom|LoopWithDelay
  (params (Index :type Integer))
  ;[1 1 1] Boucle avec 1 délai d'apparition de 2sec entre chaque ennemi
  (AI|SpawnAIFromClass "/Game/01-Blueprints/BP_Ennemy/BP_Ennemy.BP_Ennemy_C" 0 (Transformation|GetWorldLocation (Variables|Default|GetBillboard)) "0, 0, 0" true 0)
  (bind _result (Math|Integer|IncrementInt Index)
    (:%20%20
      (if (< _result (Variables|Default|GetNumbersOfEnnemies))
        (Utilities|FlowControl|Delay 1.0)
        (CallFunction|LoopwithDelay Index)
        (if (Variables|Default|GetIsReset)
          (CallFunction|ResetbyPortail))))))

(event Custom|ResetByPortail
  ;[1 1 1] Reset de la wave à 0 zéro et destruction des ennemies
  (Variables|Default|SetIsReset true)
  (Variables|Default|SetNumbersOfEnnemies 3)
  (bind _outactors (Actor|GetAllActorsOfClass "/Game/01-Blueprints/BP_Ennemy/BP_Ennemy.BP_Ennemy_C"))
  (for _array_element _outactors
    (Actor|DestroyActor _array_element)))

(event Custom|WaveEnd
  ;[1 1 1] Si le nombres d'ennemies restant est égal à 0 attendre puis lancer la vague suivante
  (if (<= (Variables|Default|GetEnnemiesLeft) 0)
    (bind _output_get (Variables|Default|SetNumbersOfEnnemies (+ (Variables|Default|GetNumbersOfEnnemies) 2)))
    (Variables|Default|SetEnnemiesLeft _output_get)
    (if (Variables|Default|GetIsReset)
      (CallFunction|ResetbyPortail)
      (else
        (Utilities|FlowControl|Delay 5.0)
        (CallFunction|LoopwithDelay)))))

(event EventBeginPlay
  ;[1 1 1] Setup du nombres d'ennemies restant au start
  (Variables|Default|SetEnnemiesLeft (Variables|Default|GetNumbersOfEnnemies)))

(event Input|KeyboardEvents|T
  (params (Key :type Key%20Structure :default "None"))
  ;[1 1 1] Lancement de la 1ere vague
  (:Pressed
    (Variables|Default|SetIsReset false)
    (CallFunction|LoopwithDelay)))

(event Input|KeyboardEvents|R
  (params (Key :type Key%20Structure :default "None"))
  ;[1 1 1] Appel Event Reset
  (:Pressed
    (CallFunction|ResetbyPortail)))

(fn ConstructionScript)