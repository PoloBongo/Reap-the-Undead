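; BP_Ennemy is a zombie enemy that chases and damages the player and counts toward the current wave.
; Tick copies its health to a widget bar; an empty bar destroys it, decrements BP_Vague's EnnemiesLeft and calls WaveEnd.
; PawnSensing sighting starts an AIMoveTo toward the player, with no re-issue on completion.
; Reaching the player calls PlayerDead, applies damage through PlayerHealthComponent and triggers AttackTrigger's AnimDegat.
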(event OnSeePawn(PawnSensing)
  (params (Pawn :type Pawn%20Object%20Reference))
  (Variables|Default|SetisFollowingPlayer true)
  (CallFunction|FollowPlayer))

(event Custom|FollowPlayer
  (if (Variables|Default|GetisFollowingPlayer)
    (AI|AIMoveTo self "0, 0, 0" (Game|GetPlayerCharacter 0) 5.0 false
      (:OnSuccess
        (bind _returnvalue (Actor|GetActorOfClass "/Game/ThirdPerson/Blueprints/BP_ThirdPersonCharacter.BP_ThirdPersonCharacter_C"))
        (Default|PlayerDead _returnvalue)
        (Class|PlayerHealthComponent|EnnemyDamage (Actor|GetComponentbyClass _returnvalue "/Script/ReapTheUndead.PlayerHealthComponent") 1.0)
        (bind _returnvalue_2 (Actor|GetActorOfClass "/Game/01-Blueprints/BP_Attack/AttackTrigger.AttackTrigger_C"))
        (Default|AnimDegat _returnvalue_2)))))

(event EventTick
  (params (DeltaSeconds :type Float%20%28single-precision%29))
  (bind _aswg_health_bar (Utilities|Casting|CastToWG_HealthBar (UserInterface|GetWidget (Variables|Default|GetWidget))))
  (Progress|SetPercent (Variables|/Game/02-UI/Ennemy/WG_HealthBar.WG_HealthBar_C|GetProgressBar_0 _aswg_health_bar) (/ (Variables|/Script/ReapTheUndead.HealthComponent|GetHealth (Variables|Default|GetHealth)) 1e+02))
  (Variables|Default|SetIsDead (<= (Variables|/Script/UMG.ProgressBar|GetPercent (Variables|/Game/02-UI/Ennemy/WG_HealthBar.WG_HealthBar_C|GetProgressBar_0 _aswg_health_bar)) 0.0))
  (if (Variables|Default|GetIsDead)
    (Actor|DestroyActor self)
    (bind _returnvalue (Actor|GetActorOfClass "/Game/01-Blueprints/BP_Ennemy/BP_Vague.BP_Vague_C"))
    (bind _result (Math|Integer|DecrementInt (Variables|/Game/01-Blueprints/BP_Ennemy/BP_Vague.BP_Vague_C|GetEnnemiesLeft _returnvalue))
      (:%20%20
        (Variables|/Game/01-Blueprints/BP_Ennemy/BP_Vague.BP_Vague_C|SetEnnemiesLeft _returnvalue _result)
        (Default|WaveEnd _returnvalue)))))

(event EventBeginPlay
  (Variables|/Script/Engine.CharacterMovementComponent|SetMaxWalkSpeed (Variables|Character|GetCharacterMovement) (Variables|Default|GetSpeed))
  (Components|Animation|PlayAnimation (Variables|Character|GetMesh) "/Game/06-Animations/Sk_Ennemy/SK_ZombieMove.SK_ZombieMove" true))

(fn ConstructionScript)