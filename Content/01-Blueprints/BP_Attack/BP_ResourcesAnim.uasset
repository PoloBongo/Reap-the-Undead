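; Handles the player's gathering animations for timber and mining when the Interact input fires.
; If ResourcesManager allows either action, it notifies the manager, spawns an axe or pickaxe on the character's right-hand socket without collision, and plays the matching montage.
; The axe is destroyed and IsPlaying cleared when its montage completes.
; The pickaxe branch does both immediately after starting its montage, without waiting for completion.
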(event Input|EnhancedActionEvents|EnhancedInputActionIA_Interact
  (params (ActionValue :type Boolean) (ElapsedSeconds :type Float%20%28double-precision%29) (TriggeredSeconds :type Float%20%28double-precision%29) (InputAction :type Input%20Action%20Object%20Reference :default "/Game/ThirdPerson/Input/Actions/IA_Interact.IA_Interact"))
  (bind _spawn_transform (Variables|Default|GetSpawn%20Transform))
  (bind _resourcesmanager (Variables|Default|GetResourcesManager))
  (Utilities|IsValid _resourcesmanager
    (:Is%20Valid
      (Utilities|FlowControl|Sequence
        (:then_0
          (if (Variables|/Script/ReapTheUndead.ResourcesManager|GetCanPlayAnimationTimber _resourcesmanager)
            (Class|ResourcesManager|OnPlayAnimationTimber _resourcesmanager)
            (bind _returnvalue (Actor|GetActorOfClass "/Game/ThirdPerson/Blueprints/BP_ThirdPersonCharacter.BP_ThirdPersonCharacter_C"))
            (bind _returnvalue_2 (Game|SpawnActorfromClass "/Game/01-Blueprints/BP_Attack/Axe.Axe_C" _spawn_transform "AlwaysSpawn" "MultiplyWithRoot" 0 0))
            (bind _output_get (Variables|Default|SetNewVar _returnvalue_2))
            (Collision|SetCollisionEnabled (Variables|/Game/01-Blueprints/BP_Attack/Axe.Axe_C|Getaxe _output_get) "NoCollision")
            (Transformation|AttachComponentToComponent (Variables|/Script/Engine.Actor|GetRootComponent _output_get) (Variables|/Script/Engine.Character|GetMesh _returnvalue) "hand_r" "KeepRelative" "KeepRelative" "KeepRelative" true)
            (Variables|Default|Setis%20playing true)
            (Animation|Montage|PlayMontage (Variables|/Script/Engine.Character|GetMesh _returnvalue) "/Game/06-Animations/SK_Attack/Lumberjack.Lumberjack"
              (:OnCompleted
                (Actor|DestroyActor (Variables|Default|GetNewVar))
                (Variables|Default|Setis%20playing false)))))
        (:then_1
          (if (Variables|/Script/ReapTheUndead.ResourcesManager|GetCanPlayAnimationMiner _resourcesmanager)
            (Class|ResourcesManager|OnPlayAnimationMiner _resourcesmanager)
            (bind _returnvalue_3 (Actor|GetActorOfClass "/Game/ThirdPerson/Blueprints/BP_ThirdPersonCharacter.BP_ThirdPersonCharacter_C"))
            (bind _returnvalue_4 (Game|SpawnActorfromClass "/Game/01-Blueprints/BP_Attack/Pickaxe.Pickaxe_C" _spawn_transform "AlwaysSpawn" "MultiplyWithRoot" 0 0))
            (bind _output_get_2 (Variables|Default|SetNewVar_0 _returnvalue_4))
            (Collision|SetCollisionEnabled (Variables|/Game/01-Blueprints/BP_Attack/Pickaxe.Pickaxe_C|Getbasicpickaxe_fbx _output_get_2) "NoCollision")
            (Transformation|AttachComponentToComponent (Variables|/Script/Engine.Actor|GetRootComponent _output_get_2) (Variables|/Script/Engine.Character|GetMesh _returnvalue_3) "hand_r" "KeepRelative" "KeepRelative" "KeepRelative" true)
            (Variables|Default|Setis%20playing true)
            (Animation|Montage|PlayMontage (Variables|/Script/Engine.Character|GetMesh _returnvalue_3) "/Game/06-Animations/SK_Attack/SK_Miner_Montage.SK_Miner_Montage"
              (:then
                (Actor|DestroyActor (Variables|Default|GetNewVar_0))
                (Variables|Default|Setis%20playing false)))))))))

(fn ConstructionScript)