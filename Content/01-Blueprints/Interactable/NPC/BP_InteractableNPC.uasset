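; BP_InteractableNPC is an interactable NPC Blueprint that stores references to inventory, notification and crafting UI objects.
; On BeginPlay it finds the BP_NotificationManager actor and caches it.
; Setter events receive and store the inventory system, wrap box, send button, craft border and left and right arrows.
; The graph contains no interaction or crafting logic, and the construction script is empty.
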(event Custom|SetArrowRight
  (params (NewParam :type Button%20Object%20Reference))
  (Variables|Default|SetArrowRight NewParam))

(event Custom|SetInventorySystemEvent
  (params (NewParam :type BP%20Inventory%20System%20Object%20Reference))
  (Variables|Default|SetInventorySystem NewParam))

(event Custom|SetCraftingBtn
  (params (NewParam :type Button%20Object%20Reference))
  (Variables|Default|SetSendButton NewParam))

(event Custom|SetWrapBoxEvent
  (params (NewParam :type Wrap%20Box%20Object%20Reference))
  (Variables|Default|SetWrapBox NewParam))

(event Custom|SetCraftBorder
  (params (NewParam :type Border%20Object%20Reference))
  (Variables|Default|SetCraftBorder NewParam))

(event Custom|SetArrowLeft
  (params (NewParam :type Button%20Object%20Reference))
  (Variables|Default|SetArrowLeft NewParam))

(event EventBeginPlay
  (bind _returnvalue (Actor|GetActorOfClass "/Game/01-Blueprints/Notification/BP_NotificationManager.BP_NotificationManager_C"))
  (Variables|Default|SetNotification _returnvalue))

(fn ConstructionScript)