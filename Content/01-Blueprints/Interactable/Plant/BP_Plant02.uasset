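; BP_Plant02 is an interactable plant actor with a world-space widget prompting the player, in French, to press E to plant.
; Tick shows the widget only within MaxDistance of the camera and rotates it on yaw to face the player.
; An OnTextChanged dispatcher updates the widget's text.
; On BeginPlay it sets the prompt and registers itself with the third-person character's ABP_Manny Animation Blueprint through SetupBPPlan2.
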(event Custom|OnTextChanged_Event
  (params (NewText :type String))
  (bind _aswg_interactable_object (Utilities|Casting|CastToWG_InteractableObject (UserInterface|GetWidget (Variables|Default|GetUserWidget))))
  (Variables|/Game/02-UI/WG_InteractableObject.WG_InteractableObject_C|SetStringValue _aswg_interactable_object NewText))

(event EventBeginPlay
  (Variables|Default|SetUIUserInteract (UserInterface|GetWidget (Variables|Default|GetUserWidget)))
  (Variables|Default|SetHarvestWidgetUI 0)
  (EventDispatchers|AssignOnTextChanged (delegate Custom|OnTextChanged_Event))
  (CallFunction|OnTextChangedEvent "Appuyez sur [E] pour planter")
  (bind _returnvalue (Actor|GetActorOfClass "/Game/ThirdPerson/Blueprints/BP_ThirdPersonCharacter.BP_ThirdPersonCharacter_C"))
  (bind _asabp_manny (Utilities|Casting|CastToABP_Manny (Components|SkeletalMesh|GetAnimInstance (Variables|/Script/Engine.Character|GetMesh _returnvalue))))
  (Default|SetupBPPlan2 _asabp_manny self))

(event EventTick
  (params (DeltaSeconds :type Float%20%28single-precision%29))
  (bind _returnvalue (Game|GetPlayerCameraManager 0))
  (bind _userwidget (Variables|Default|GetUserWidget))
  (bind _userwidget_2 (Variables|Default|GetUserWidget))
  (bind _returnvalue_2 (Camera|GetCameraLocation _returnvalue))
  (bind _returnvalue_3 (Transformation|GetWorldLocation _userwidget_2))
  ;[1 1 1] Permet que le text reste orienter face au player + si le joueur est hors de porté, le text ne s'affiche plus
  (Rendering|SetVisibility _userwidget (< (Math|Vector|Distance(Vector) _returnvalue_2 _returnvalue_3) (Variables|Default|GetmaxDistance)) false)
  (Transformation|SetWorldRotation _userwidget (Math|Rotator|MakeRotator 1.8e+02 1.8e+02 (.yaw (Math|Rotator|FindLookatRotation _returnvalue_2 _returnvalue_3))) false false))

(fn ConstructionScript)