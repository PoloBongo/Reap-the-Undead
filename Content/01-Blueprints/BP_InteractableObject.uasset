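; BP_InteractableObject is a base-style interactable actor that lets the player press E while inside its trigger box.
; Overlap by the player character shows an interaction widget created at BeginPlay, applies an outline overlay material and enables input handling through a flag; leaving reverses this.
; StartTrigger runs on entry and Interact on E, both empty stubs like EndTrigger, which is never called.
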(event OnComponentBeginOverlap(Box)
  (params (OverlappedComponent :type Primitive%20Component%20Object%20Reference) (OtherActor :type Actor%20Object%20Reference) (OtherComp :type Primitive%20Component%20Object%20Reference) (OtherBodyIndex :type Integer) (bFromSweep :type Boolean) (SweepResult :type Hit%20Result%20Structure%20%28by%20ref%29))
  (if (== OtherActor (Game|GetPlayerCharacter 0))
    (UserInterface|Viewport|AddtoViewport (Variables|Default|GetInteractWidget) 0)
    (Variables|Default|SetplayerTrigger true)
    (Rendering|Material|SetOverlayMaterial (Variables|Default|GetMesh) "/Game/03_Material/M_Outline.M_Outline" :!class /Script/Engine.MeshComponent)
    (CallFunction|StartTrigger)))

(event OnComponentEndOverlap(Box)
  (params (OverlappedComponent :type Primitive%20Component%20Object%20Reference) (OtherActor :type Actor%20Object%20Reference) (OtherComp :type Primitive%20Component%20Object%20Reference) (OtherBodyIndex :type Integer))
  (if (== (Game|GetPlayerCharacter 0) OtherActor)
    (Widget|RemovefromParent (Variables|Default|GetInteractWidget))
    (Variables|Default|SetplayerTrigger false)
    (Rendering|Material|SetOverlayMaterial (Variables|Default|GetMesh) 0 :!class /Script/Engine.MeshComponent)))

(event EventBeginPlay
  (bind _returnvalue (UserInterface|CreateWidget "/Game/02_UI/WG_InteractableObject.WG_InteractableObject_C"))
  (Variables|Default|SetInteractWidget _returnvalue))

(event Input|KeyboardEvents|E
  (params (Key :type Key%20Structure))
  (:Pressed
    (if (Variables|Default|GetplayerTrigger)
      (CallFunction|Interact))))

(fn ConstructionScript)

(fn StartTrigger)

(fn EndTrigger)

(fn Interact)