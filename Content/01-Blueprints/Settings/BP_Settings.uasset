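; BP_Settings is an actor that owns and toggles the WG_Settings settings menu.
; On BeginPlay it creates the widget, adds it to the viewport and hides it.
; The B key shows the widget with the mouse cursor and UI-only input locked to the viewport.
; A CloseUI event hides the cursor and restores game-only input, without changing the widget's visibility itself.
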(event Custom|CloseUI
  (bind _returnvalue (Game|GetPlayerController 0))
  (Variables|/Script/Engine.PlayerController|SetbShowMouseCursor _returnvalue false)
  (Input|SetInputModeGameOnly _returnvalue false))

(event EventBeginPlay
  (bind _returnvalue (Game|ConstructObjectfromClass "/Game/01-Blueprints/Settings/WG_Settings.WG_Settings_C"))
  (Variables|Default|SetWG_Settings _returnvalue)
  (UserInterface|Viewport|AddtoViewport (Variables|Default|GetWG_Settings) 0)
  (Default|ManageVisibility (Variables|Default|GetWG_Settings) "Hidden"))

(event Input|KeyboardEvents|B
  (params (Key :type Key%20Structure :default "None"))
  (bind _returnvalue (Game|GetPlayerController 0))
  (:Pressed
    (Variables|/Script/Engine.PlayerController|SetbShowMouseCursor _returnvalue true)
    (Input|SetInputModeUIOnly _returnvalue (Variables|Default|GetWG_Settings) "LockAlways" false)
    (Default|ManageVisibility (Variables|Default|GetWG_Settings) "Visible")))

(fn ConstructionScript)