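; BP_DropItem0 is a dropped inventory item actor that registers itself with the inventory system.
; On BeginPlay it finds BP_InventorySystem, adds itself to its DropItemInstances list, and caches BP_NotificationManager.
; When destroyed, it finds BP_ThirdPersonCharacter, calls SetDropItem on its DetectionDrop, then stores the character reference.
; All references come from GetActorOfClass lookups without validity checks.
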(event EventBeginPlay
  (bind _returnvalue (Actor|GetActorOfClass "/Game/01-Blueprints/Inventory/BP_InventorySystem.BP_InventorySystem_C"))
  (bind _output_get (Variables|Default|SetInventorySystem _returnvalue))
  (Utilities|Array|Add (Variables|/Script/ReapTheUndead.InventorySystem|GetDropItemInstances _output_get) self)
  (bind _returnvalue_2 (Actor|GetActorOfClass "/Game/01-Blueprints/Notification/BP_NotificationManager.BP_NotificationManager_C"))
  (Variables|Default|SetGameNotificationManager _returnvalue_2))

(event EventDestroyed
  (bind _returnvalue (Actor|GetActorOfClass "/Game/ThirdPerson/Blueprints/BP_ThirdPersonCharacter.BP_ThirdPersonCharacter_C"))
  (Class|DetectionDrop|SetDropItem (Variables|/Game/ThirdPerson/Blueprints/BP_ThirdPersonCharacter.BP_ThirdPersonCharacter_C|GetDetectionDrop _returnvalue) 0)
  (Variables|Default|SetReapTheUndeadCharacter _returnvalue))

(fn ConstructionScript)