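; Double door Blueprint with a sliding lock and two leaves that swing open and closed.
; A lock timeline drives the lock mesh's position and pitch, and a door timeline yaws the leaves in opposite directions.
; Unlock and open events play these timelines forward, while lock and close events reverse them.
; The Construction Script calls these events from two booleans, with LockedDoor triggering unlock and OpenedDoor triggering close when true.
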(event Custom|CloseDoor
  (bind _dooranimation (Timeline|DoorAnimation ReverseFromEnd)
    (:Update
      (Transformation|SetRelativeRotation (Variables|Default|GetSM_DoorLeft) (Math|Rotator|MakeRotator 0.0 0.0 (* _dooranimation -1.0)) false false)
      (Transformation|SetRelativeRotation (Variables|Default|GetSM_DoorRight) (Math|Rotator|MakeRotator 0.0 0.0 _dooranimation) false false))))

(event Custom|OpenDoor
  (bind _dooranimation (Timeline|DoorAnimation PlayFromStart)
    (:Update
      (Transformation|SetRelativeRotation (Variables|Default|GetSM_DoorLeft) (Math|Rotator|MakeRotator 0.0 0.0 (* _dooranimation -1.0)) false false)
      (Transformation|SetRelativeRotation (Variables|Default|GetSM_DoorRight) (Math|Rotator|MakeRotator 0.0 0.0 _dooranimation) false false))))

(event Custom|UnlockDoor
  (bind _animmation (Timeline|LockAnimation PlayFromStart)
    (:Update
      (Transformation|SetRelativeTransform (Variables|Default|GetSM_DoorLock) (Math|Transform|MakeTransform (Math|Vector|MakeVector (.x _animmation) -4.0665 115.695129) (Math|Rotator|MakeRotator 0.0 (.y _animmation) 0.0) "1.000000,1.000000,1.000000") false false))))

(event Custom|LockDoor
  (bind _animmation (Timeline|LockAnimation ReverseFromEnd)
    (:Update
      (Transformation|SetRelativeTransform (Variables|Default|GetSM_DoorLock) (Math|Transform|MakeTransform (Math|Vector|MakeVector (.x _animmation) -4.0665 115.695129) (Math|Rotator|MakeRotator 0.0 (.y _animmation) 0.0) "1.000000,1.000000,1.000000") false false))))

(fn ConstructionScript
  (Utilities|FlowControl|Sequence
    (:then_0
      (if (Variables|Default|GetLockedDoor?)
        (CallFunction|UnlockDoor)
        (else
          (CallFunction|LockDoor))))
    (:then_1
      (if (Variables|Default|GetOpenedDoor?)
        (CallFunction|CloseDoor)
        (else
          (CallFunction|OpenDoor))))))